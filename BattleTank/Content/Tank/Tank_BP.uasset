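; Player-controllable tank Blueprint that wires input to aiming and movement components.
; On BeginPlay it hands the turret and barrel to TankAiming and both tracks to TankMovement.
; Forward and turn axes feed TankMovement as intents, while Fire calls TankAiming.
; Aim axes rotate the azimuth gimbal in yaw and the spring arm in pitch directly, using raw axis values without delta-time scaling.
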(event EventBeginPlay
  (Class|TankAimingComponent|Initialise (Variables|Default|GetTankAiming) (Variables|Default|GetTurret) (Variables|Default|GetBarrel))
  (Class|TankMovementComponent|Initialise (Variables|Default|GetTankMovement) (Variables|Default|GetLeftTrack) (Variables|Default|GetRightTrack)))

(event Input|ActionEvents|InputActionFire
  (params (Key :type Key%20Structure))
  ;[1 1 1] Aiming input binding
  (:Pressed
    (Class|TankAimingComponent|Fire (Variables|Default|GetTankAiming))))

(event Input|AxisEvents|InputAxisAimAzimuth
  (params (AxisValue :type Float%20%28single-precision%29))
  ;[1 1 1] Aiming input binding
  (Transformation|AddLocalRotation (Variables|Default|GetAximuth%20Gimble) (Math|Rotator|MakeRotator 0.0 0.0 AxisValue) false false))

(event Input|AxisEvents|InputAxisAimElevation
  (params (AxisValue :type Float%20%28single-precision%29))
  ;[1 1 1] Aiming input binding
  (Transformation|AddLocalRotation (Variables|Default|GetSpringArm) (Math|Rotator|MakeRotator 0.0 AxisValue 0.0) false false))

(event Input|AxisEvents|InputAxisRightIntent
  (params (AxisValue :type Float%20%28single-precision%29))
  ;[1 1 1] Ipnut Binding
  (Class|TankMovementComponent|IntendTurnRight (Variables|Default|GetTankMovement) AxisValue))

(event Input|AxisEvents|InputAxisForwardIntent
  (params (AxisValue :type Float%20%28single-precision%29))
  ;[1 1 1] Ipnut Binding
  (Class|TankMovementComponent|IntendMoveForward (Variables|Default|GetTankMovement) AxisValue))

(fn ConstructionScript)